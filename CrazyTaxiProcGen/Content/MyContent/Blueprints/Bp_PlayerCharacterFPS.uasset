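; First-person player character Blueprint that handles the game's pause menu.
; On BeginPlay it creates the pause widget for the first player controller, adds it to the viewport and hides it.
; The Pause input action uses an IsPaused flag to toggle widget visibility, the mouse cursor and the game's paused state.
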(event EventBeginPlay
  (bind _returnvalue (UserInterface|CreateWidget "/Game/MyContent/Widgets/WidgetPause.WidgetPause_C" (Game|GetPlayerController 0)))
  (UserInterface|Viewport|AddtoViewport _returnvalue 0)
  (Widget|SetVisibility _returnvalue "Hidden"))

(event Input|ActionEvents|InputActionPause
  (params (Key :type Key%20Structure))
  (:Pressed
    (if (Variables|Default|GetIsPaused)
      (Widget|SetVisibility (stale EventBeginPlay _returnvalue) "Hidden")
      (Variables|/Script/Engine.PlayerController|SetbShowMouseCursor (Game|GetPlayerController 0) false)
      (Game|SetGamePaused false)
      (Variables|Default|SetIsPaused false)
      (else
        (Widget|SetVisibility (stale EventBeginPlay _returnvalue) "Visible")
        (Variables|/Script/Engine.PlayerController|SetbShowMouseCursor (Game|GetPlayerController 0) true)
        (Game|SetGamePaused true)
        (Variables|Default|SetIsPaused true)))))

(fn ConstructionScript)