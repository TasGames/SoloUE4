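; Maze actor that procedurally builds a square grid maze in its construction script, using instanced meshes for border, walls and path floor.
; A seeded depth-first carve steps two tiles at a time, recording the tiles between as bridges and backtracking through unchecked path tiles.
; Bridges become path as it unwinds, then untouched tiles become walls.
; Optionally, random qualifying walls become paths to create loops before the tiles are spawned.
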(event EventBeginPlay)

(event Collision|EventActorBeginOverlap
  (params (OtherActor :type Actor%20Object%20Reference)))

(event EventTick
  (params (DeltaSeconds :type Float%20%28single-precision%29)))

(fn ConstructionScript
  (CallFunction|PopulateBoarder (Variables|Default|GetSize) (Variables|Default|GetBoarderTiles))
  (if (Variables|Default|GetShowBoarder)
    (Utilities|SpawnImstances (Variables|Default|GetBoarderTiles) (Variables|Default|GetSize) (Variables|Default|GetTileSize) "8.000000,8.000000,16.000000" (Variables|Default|GetWall)
      (:Finished
        _)))
  (if (Variables|Default|GetShowMaze)
    (CallFunction|SetInitialTile)
    (while (Variables|Default|GetCurrentFreeSide) :!label _label
      (CallFunction|PickNearbyTile))
    (Utilities|Array|Add (Variables|Default|GetCheckedTiles) (Variables|Default|GetCurrentTile))
    (CallFunction|BackTrack)
    (Utilities|ConvertLastBridge
      (:BridgesLeft
        (goto _label))
      (:NoBridgesLeft
        (CallFunction|PopulateWalls)
        (if (Variables|Default|GetAllowLoopPaths)
          (CallFunction|AddLoopPaths))
        (Utilities|SpawnImstances (Variables|Default|GetPathTiles) (Variables|Default|GetSize) (Variables|Default|GetTileSize) "8.000000,8.000000,0.125000" (Variables|Default|GetWall)
          (:Finished
            (Utilities|SpawnImstances (Variables|Default|GetWallTiles) (Variables|Default|GetSize) (Variables|Default|GetTileSize) "8.000000,8.000000,10.000000" (Variables|Default|GetWall))))))))

(fn PopulateBoarder
  (params (Size :type Integer) (BoarderArray :type Array%20of%20Integers))
  (LocalVariables|SetL_Size Size)
  ;[1 1 1] North
  (for _index (range 0 (- (LocalVariables|GetL_Size) 1))
    (Utilities|Array|Add BoarderArray _index))
  ;[1 1 1] East
  (for _index_2 (range 1 (- (LocalVariables|GetL_Size) 2))
    (Utilities|Array|Add BoarderArray (+ (* _index_2 (LocalVariables|GetL_Size)) (- (LocalVariables|GetL_Size) 1))))
  ;[1 1 1] South
  (for _index_3 (range 1 (LocalVariables|GetL_Size))
    (Utilities|Array|Add BoarderArray (+ (- _index_3 1) (* (LocalVariables|GetL_Size) (- (LocalVariables|GetL_Size) 1)))))
  ;[1 1 1] West
  (for _index_4 (range 1 (- (LocalVariables|GetL_Size) 2))
    (Utilities|Array|Add BoarderArray (* _index_4 (LocalVariables|GetL_Size)))))

(fn SetInitialTile
  (Variables|Default|SetCurrentTile (+ (Variables|Default|GetSize) 1))
  (Utilities|Array|Add (Variables|Default|GetPathTiles) (Variables|Default|GetCurrentTile)))

(fn AddBridge&PathTile
  (params (PathTile :type Integer) (BridgeTile :type Integer))
  (Utilities|Array|Add (Variables|Default|GetPathTiles) PathTile)
  (Variables|Default|SetCurrentTile PathTile)
  (Utilities|Array|Add (Variables|Default|GetBridgeTiles) BridgeTile))

(fn PickNearbyTile
  (bind _currenttile (Variables|Default|GetCurrentTile))
  (bind _currenttile_2 (Variables|Default|GetCurrentTile))
  (bind _size (Variables|Default|GetSize))
  (bind _currenttile_3 (Variables|Default|GetCurrentTile))
  (bind _size_2 (Variables|Default|GetSize))
  (bind _currenttile_4 (Variables|Default|GetCurrentTile))
  (bind (_tileinarrays _pathtile _bridgetile) (Utilities|CheckNorthTile _currenttile _size_2 true))
  (bind (_tileinarrays_2 _pathtile_2 _bridgetile_2) (Utilities|CheckEastTile _currenttile_3 false))
  (bind (_tileinarrays_3 _pathtile_3 _bridgetile_3) (Utilities|CheckEastTile _currenttile_4 true))
  (bind (_tileinarrays_4 _pathtile_4 _bridgetile_4) (Utilities|CheckNorthTile _currenttile_2 _size false))
  (switch int (Math|Random|RandomIntegerinRangefromStream 0 3 (Variables|Default|GetRandomStream))
    (:0
      (if _tileinarrays_4 :!label _label
        (Utilities|CycleCounter (LocalVariables|GetCycleCount) 4
          (:True
            (if _tileinarrays :!label _label_2
              (Utilities|CycleCounter (LocalVariables|GetCycleCount) 4
                (:True
                  (if _tileinarrays_2 :!label _label_3
                    (Utilities|CycleCounter (LocalVariables|GetCycleCount) 4
                      (:True
                        (if _tileinarrays_3 :!label _label_4
                          (Utilities|CycleCounter (LocalVariables|GetCycleCount) 4
                            (:True
                              (goto _label))
                            (:False
                              (Variables|Default|SetCurrentFreeSide false :!label _label_5)))
                          (else
                            (CallFunction|AddBridge&PathTile _pathtile_3 _bridgetile_3))))
                      (:False
                        (goto _label_5)))
                    (else
                      (CallFunction|AddBridge&PathTile _pathtile_2 _bridgetile_2))))
                (:False
                  (goto _label_5)))
              (else
                (CallFunction|AddBridge&PathTile _pathtile _bridgetile))))
          (:False
            (goto _label_5)))
        (else
          (CallFunction|AddBridge&PathTile _pathtile_4 _bridgetile_4))))
    (:1
      (goto _label_3))
    (:2
      (goto _label_2))
    (:3
      (goto _label_4)))
  (return))

(fn BackTrack
  (bind _arrayelement (Utilities|ForEachLoopwithBreakRev (Variables|Default|GetPathTiles) :!label _label)
    (:LoopBody
      (if (not (Utilities|Array|ContainsItem (Variables|Default|GetCheckedTiles) _arrayelement))
        (Variables|Default|SetCurrentTile _arrayelement)
        (goto _label Break)))))

(fn PopulateWalls
  (bind _size (Variables|Default|GetSize))
  (for _index (range 0 (- (* _size _size) 1))
    (if (not (Utilities|CheckTileArrays _index))
      (Utilities|Array|Add (Variables|Default|GetWallTiles) _index))))

(fn AddLoopPaths
  (LocalVariables|SetLoopPathsAdded 0)
  (LocalVariables|SetLoopPath (Utilities|GetRandomElement (Variables|Default|GetWallTiles) (Variables|Default|GetRandomStream)) :!label _label)
  (if (Utilities|TileSurrounded (LocalVariables|GetLoopPath))
    _
    (else
      (Utilities|Add&RemoveItem (LocalVariables|GetLoopPath) (Variables|Default|GetPathTiles) (Variables|Default|GetWallTiles)
        (:Out
          (LocalVariables|SetLoopPathsAdded (+ (LocalVariables|GetLoopPathsAdded) 1))))))
  (if (< (LocalVariables|GetLoopPathsAdded) (Variables|Default|GetMaxLoopPaths))
    (goto _label)))